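; BP_Weapon is a grippable weapon actor for motion controllers, with a placeholder trace on input.
; Gripping turns off StaticMesh physics and snaps the root to the controller's Palm socket.
; Release re-enables physics and calls detach on the releasing controller component, not the weapon root.
; Input handling references the right grip key, then runs a debug-drawn Visibility multi-line trace and prints a message, leaving hits unused.
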(event EventBeginPlay)

(event Collision|EventActorBeginOverlap
  (params (OtherActor :type Actor%20Object%20Reference)))

(event EventTick
  (params (DeltaSeconds :type Float%20%28single-precision%29)))

(event EventOnInput
  (params (Key :type Key%20Structure) (KeyEvent :type EInputEvent%20Enum :default "IE_Pressed"))
  (Class|GrippableActor|OnInput "MotionController_Right_Grip1" KeyEvent)
  (Collision|MultiLineTraceByChannel "0, 0, 0" "0, 0, 0" "TraceTypeQuery1" false 0 "ForDuration")
  (Development|PrintString "BP_Weapon_Trace" true true "(R=1.000000,G=0.000000,B=0.026949,A=1.000000)"))

(event EventOnGripRelease
  (params (ReleasingController :type Grip%20Motion%20Controller%20Component%20Object%20Reference) (GripInformation :type BP%20Actor%20Grip%20Information%20Structure%20%28by%20ref%29) (bWasSocketed :type Boolean))
  (Physics|SetSimulatePhysics (Variables|Default|GetStaticMesh) true)
  (Transformation|DetachFromComponent ReleasingController "KeepWorld" "KeepWorld" "KeepWorld" true))

(event EventOnGrip
  (params (GrippingController :type Grip%20Motion%20Controller%20Component%20Object%20Reference) (GripInformation :type BP%20Actor%20Grip%20Information%20Structure%20%28by%20ref%29))
  (Physics|SetSimulatePhysics (Variables|Default|GetStaticMesh) false)
  (Transformation|AttachComponentToComponent (Variables|Default|GetRoot) GrippingController "Palm" "SnapToTarget" "SnapToTarget" "SnapToTarget" true))

(fn ConstructionScript)