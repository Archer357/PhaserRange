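; BP_Physics is a skeletal mesh object that can be picked up and dropped with partial ragdoll physics.
; Pickup disables simulation, attaches the root to the given component keeping world transform, then simulates bodies below an anchor bone.
; The anchor is the physics asset bone closest to the mesh component's own world location, not a passed grab point.
; Drop re-enables simulation from that bone down and mesh-wide, then detaches the actor.
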(event EventPickup
  (params (AttachTo :type Scene%20Component%20Object%20Reference))
  ;[0 0 0] Handles picking up the object. It attaches the object to the parent, finds the nearest bone on the object and then simulates physics on bones below that object in the hierarchy.
  (Physics|SetSimulatePhysics (Variables|SkeletalMeshActor|GetSkeletalMeshComponent) false)
  (Transformation|AttachComponentToComponent (VehicleSound|GetRootComponent) AttachTo "None" "KeepWorld" "KeepWorld" "KeepWorld" false)
  (CallFunction|SimulateBelowBone))

(event EventDrop
  ;[0 0 0] Handles dropping the object. Simulate All is the same as SimulateBelowBone, but with Self included.
  (CallFunction|SimulateAll)
  (Physics|SetSimulatePhysics (Variables|SkeletalMeshActor|GetSkeletalMeshComponent) true)
  (Transformation|DetachFromActor "KeepWorld" "KeepWorld" "KeepWorld"))

(fn ConstructionScript)

(fn SimulateAll
  (bind _skeletalmeshcomponent (Variables|SkeletalMeshActor|GetSkeletalMeshComponent))
  (Class|SkeletalMeshComponent|SetAllBodiesBelowSimulatePhysics (Variables|SkeletalMeshActor|GetSkeletalMeshComponent) (Utilities|Name|MakeLiteralName (.BoneName (Class|SkeletalMeshComponent|GetClosestPointonPhysicsAsset _skeletalmeshcomponent (Transformation|GetWorldLocation _skeletalmeshcomponent)))) true true))

(fn SimulateBelowBone
  (bind _skeletalmeshcomponent (Variables|SkeletalMeshActor|GetSkeletalMeshComponent))
  (Class|SkeletalMeshComponent|SetAllBodiesBelowSimulatePhysics (Variables|SkeletalMeshActor|GetSkeletalMeshComponent) (Utilities|Name|MakeLiteralName (.BoneName (Class|SkeletalMeshComponent|GetClosestPointonPhysicsAsset _skeletalmeshcomponent (Transformation|GetWorldLocation _skeletalmeshcomponent)))) true false))